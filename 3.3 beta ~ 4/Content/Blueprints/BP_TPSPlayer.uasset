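; Third-person shooter player Blueprint that handles the player's UI on top of inherited character logic.
; BeginPlay creates the HUD and, after a brief delay, fills its HP ratio and text through UIctrlHP.
; Grenade toggles update the HUD's weapon display, and game over calls the parent before showing a game-over screen.
; The sniper input event is empty; its scope widget and FOV zoom nodes are disconnected.
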(event `self.ReceiveBeginPlay`
  (bind _returnvalue (`|CreateWidget` "/Game/3-3-7-UMG/UI_Screen.UI_Screen_C" (`GameplayStatics.GetPlayerController` 0)))
  (bind _output_get (set `self.uiScreen` _returnvalue))
  (`UserWidget.AddToViewport` _output_get 0)
  (`KismetSystemLibrary.Delay` 0.05)
  (`self.UIctrlHP`))

(event `EnhancedInput|/Game/Input/IA_Sniper`
  (params (ActionValue :type Boolean) (ElapsedSeconds :type "Float (double-precision)") (TriggeredSeconds :type "Float (double-precision)") (InputAction :type "InputAction Object Reference" :default "/Game/Input/IA_Sniper.IA_Sniper")))

(event `self.OnGameOver`
  (`parent.OnGameOver`)
  (bind _returnvalue (`|CreateWidget` "/Game/3-3-7-UMG/UI_GameOver.UI_GameOver_C" (`GameplayStatics.GetPlayerController` 0)))
  (`UserWidget.AddToViewport` _returnvalue 0))

(event `self.OnUsingGrenade`
  (params (isGrenade :type Boolean))
  (bind _uiscreen (`self.uiScreen`))
  (`/Engine/EditorBlueprintResources/StandardMacros.IsValid` _uiscreen
    (:`Is Valid`
      (set `/Game/3-3-7-UMG/UI_Screen.isGreneded` isGrenade _uiscreen)
      (`/Game/3-3-7-UMG/UI_Screen.SwapWeapon` _uiscreen))))

(fn `UIctrlHP`
  (set `/Game/3-3-7-UMG/UI_Screen.hpRatio` (/ (`KismetMathLibrary.Conv_IntToDouble` (`self.hp`)) (`KismetMathLibrary.Conv_IntToDouble` (`self.initialHp`))) (`self.uiScreen`))
  (set `/Game/3-3-7-UMG/UI_Screen.hpString` (`KismetStringLibrary.Concat_StrStr` (`KismetStringLibrary.Conv_IntToString` (`self.hp`)) "/" (`KismetStringLibrary.Conv_IntToString` (`self.initialHp`))) (`self.uiScreen`)))

(fn `UserConstructionScript`)