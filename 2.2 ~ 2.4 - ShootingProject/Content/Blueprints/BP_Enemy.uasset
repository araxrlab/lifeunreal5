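; BP_Enemy is an enemy actor that flies in a straight line and ends the game when it overlaps the player.
; On BeginPlay it either aims once at BP_Player or keeps its forward vector, though the TraceRate roll spans zero to zero, so any non-negative rate aims.
; Tick moves it along that direction at MoveSpeed without sweeping.
; Overlap destroys the player, spawns an emitter, shows the game-over widget and cursor, and pauses.
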(event `self.ReceiveBeginPlay`
  (if (<= (`KismetMathLibrary.RandomFloatInRange` 0.0) (`self.TraceRate`))
    (bind _returnvalue (`GameplayStatics.GetActorOfClass` "/Game/Blueprints/BP_Player.BP_Player_C"))
    (`/Engine/EditorBlueprintResources/StandardMacros.IsValid` _returnvalue
      (:`Is Valid`
        (bind _output_get (set `self.Direction` (`KismetMathLibrary.Normal` (- (`self.K2_GetActorLocation` _returnvalue) (`self.K2_GetActorLocation`)))))
        (`self.K2_SetActorRotation` (`KismetMathLibrary.MakeRotFromXZ` _output_get (`self.GetActorUpVector`)))))
    (else
      (set `self.Direction` (`self.GetActorForwardVector`)))))

(event `self.ReceiveTick`
  (params (DeltaSeconds :type "Float (single-precision)"))
  (`self.K2_SetActorLocation` (+ (`self.K2_GetActorLocation`) (* (* (`self.Direction`) (`self.MoveSpeed`)) DeltaSeconds))))

(event `self.ReceiveActorBeginOverlap`
  (params (OtherActor :type "Actor Object Reference"))
  (bind _asbp_player (cast `/Game/Blueprints/BP_Player` OtherActor))
  (`self.K2_DestroyActor` _asbp_player)
  (`GameplayStatics.SpawnEmitterAtLocation` null (`self.K2_GetActorLocation`))
  (bind _returnvalue (`|CreateWidget` "/Game/UI/WBP_GameOverWidget.WBP_GameOverWidget_C"))
  (`UserWidget.AddToViewport` _returnvalue 0)
  (set `PlayerController.bShowMouseCursor` true (`GameplayStatics.GetPlayerController` 0))
  (`GameplayStatics.SetGamePaused` true))

(fn `UserConstructionScript`)