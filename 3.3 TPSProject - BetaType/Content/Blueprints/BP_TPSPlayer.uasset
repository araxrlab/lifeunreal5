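; BP_TPSPlayer is the third-person player Blueprint, linking the player's health, weapon and game-over events to the HUD.
; BeginPlay creates the sniper and main screen widgets, shows the main one, then after a short delay initializes the HP display and non-grenade weapon state.
; UIctrlHP pushes HP ratio and text; OnUsingGrenade triggers the widget's weapon swap.
; OnGameOver only extends the parent with a debug print, and sniper zoom logic is disconnected.
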(event `self.ReceiveBeginPlay`
  (bind _returnvalue (`|CreateWidget` "/Game/Blueprints/WBP_SniperUI.WBP_SniperUI_C"))
  (set `self.SniperUI` _returnvalue)
  (bind _returnvalue_2 (`|CreateWidget` "/Game/3-3-7-UMG/UI_Screen.UI_Screen_C" (`GameplayStatics.GetPlayerController` 0)))
  (bind _output_get (set `self.ui_Screen` _returnvalue_2))
  (`UserWidget.AddToViewport` _output_get 0)
  (`KismetSystemLibrary.Delay` 0.05)
  (`self.UIctrlHP`)
  (`self.OnUsingGrenade` false))

(event `EnhancedInput|/Game/Input/IA_Sniper`
  (params (ActionValue :type Boolean) (ElapsedSeconds :type "Float (double-precision)") (TriggeredSeconds :type "Float (double-precision)") (InputAction :type "InputAction Object Reference" :default "/Game/Input/IA_Sniper.IA_Sniper")))

(event `self.OnGameOver`
  (`parent.OnGameOver`)
  (`KismetSystemLibrary.PrintString` "Game Over!!!"))

(event `self.OnUsingGrenade`
  (params (isGrenade :type Boolean))
  (bind _ui_screen (`self.ui_Screen`))
  (`/Engine/EditorBlueprintResources/StandardMacros.IsValid` _ui_screen
    (:`Is Valid`
      (set `/Game/3-3-7-UMG/UI_Screen.isGreneded` isGrenade _ui_screen)
      (`/Game/3-3-7-UMG/UI_Screen.SwapWeapon` _ui_screen))))

(fn `UIctrlHP`
  (set `/Game/3-3-7-UMG/UI_Screen.hpRatio` (/ (`self.hp`) (`self.initialHp`)) (`self.ui_Screen`))
  (set `/Game/3-3-7-UMG/UI_Screen.hpString` (`KismetStringLibrary.Concat_StrStr` (`KismetStringLibrary.Conv_IntToString` (`self.hp`)) "/" (`KismetStringLibrary.Conv_IntToString` (`self.initialHp`))) (`self.ui_Screen`)))

(fn `UserConstructionScript`)